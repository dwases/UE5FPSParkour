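; Test cube actor that animates the luminosity of its material, which is based on the DragonBloodKatana material instance.
; The construction script creates a dynamic material instance on the static mesh.
; BeginPlay sets it fully metallic, then a timeline feeds a scaled track value into the Luminosity parameter.
; Each time the timeline finishes it reverses from the end, so later passes all run backward.
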(event `self.ReceiveBeginPlay`
  (`MaterialInstanceDynamic.SetScalarParameterValue` (`self.DynamicMaterialInstance`) "Metallic" 1.0)
  (bind (_direction _newtrack_0) (`Timeline|LuminosityTL` :!label _label)
    (:`Update`
      (`MaterialInstanceDynamic.SetScalarParameterValue` (`self.DynamicMaterialInstance`) "Luminosity" (/ _newtrack_0 48.0)))
    (:`Finished`
      (if true
        (goto _label :!via `ReverseFromEnd`)))))

(fn `UserConstructionScript`
  (bind _returnvalue (`PrimitiveComponent.CreateDynamicMaterialInstance` (`self.StaticMeshComponent`) 0 "/Game/_Testing/Materials/MaterialInstances/DragonBloodKatanaMaterialInstance.DragonBloodKatanaMaterialInstance" "None"))
  (set `self.DynamicMaterialInstance` _returnvalue))