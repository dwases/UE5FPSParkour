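; BP_OldLamp is a test lamp actor whose bulb glows dark green with pulsing luminosity.
; The construction script creates a dynamic PulsatingColor material on the LightBulb, and BeginPlay sets its color.
; The Luminosity_TL timeline drives the material's Luminosity through a sine wave added to an inverted parabola.
; The timeline plays forward once, then restarts in reverse from its end whenever it finishes.
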(event `self.ReceiveBeginPlay`
  (`MaterialInstanceDynamic.SetVectorParameterValue` (`self.DMI_Lightbulb`) "BaseColor" (struct :`R` 0.057071 :`G` 0.166667 :`B` 0.092685 :`A` 1.0))
  (bind (_direction _x_val) (`Timeline|Luminosity_TL` :!via `PlayFromStart` :!label _label)
    (:`Update`
      (`MaterialInstanceDynamic.SetScalarParameterValue` (`self.DMI_Lightbulb`) "Luminosity" (+ (+ (`KismetMathLibrary.Sin` (* _x_val 8.0)) 1.0) (+ (* (`KismetMathLibrary.MultiplyMultiply_FloatFloat` (- _x_val 1.0) 2.0) -1.0) 1.0))))
    (:`Finished`
      (goto _label :!via `ReverseFromEnd`))))

(fn `UserConstructionScript`
  (bind _returnvalue (`PrimitiveComponent.CreateDynamicMaterialInstance` (`self.LightBulb`) 0 "/Game/_Testing/Materials/BaseMaterials/PulsatingColor.PulsatingColor" "None"))
  (set `self.DMI_Lightbulb` _returnvalue))