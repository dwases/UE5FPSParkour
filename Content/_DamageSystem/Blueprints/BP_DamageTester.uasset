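; Test actor for the damage system that periodically probes what lies in front of its Cube component and reports it, without applying any damage.
; From BeginPlay, a self-repeating delay loop runs a debug-drawn sphere trace by profile along the Cube's forward vector, ignoring itself.
; Each pass prints the hit actor's name, with no check on whether the trace hit.
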(event `self.ReceiveBeginPlay`
  (bind _returnvalue (`SceneComponent.K2_GetComponentLocation` (`self.Cube`)))
  (`KismetSystemLibrary.Delay` 4.0 :!label _label)
  (bind _outhit (`KismetSystemLibrary.SphereTraceSingleByProfile` _returnvalue (+ _returnvalue (* (`SceneComponent.GetForwardVector` (`self.Cube`)) 500.0)) 40.0 "None" false (`|MakeArray` self :!type "Actor Object Reference") "ForDuration" true (struct :`R` 1.0 :`A` 1.0) (struct :`G` 1.0 :`A` 1.0) 2.0))
  (`KismetSystemLibrary.PrintString` (`KismetStringLibrary.Concat_StrStr` "Actor hit by tester: " (`KismetSystemLibrary.GetDisplayName` (`.HitActor` (`GameplayStatics.BreakHitResult` _outhit)))))
  (goto _label))

(fn `UserConstructionScript`)